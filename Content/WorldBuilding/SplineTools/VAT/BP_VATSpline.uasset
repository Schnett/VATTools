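; Spline tool actor that configures a Niagara system to spawn moving static meshes animated with Vertex Animation Textures (VAT).
; The construction script pushes the mesh, speed, spread and spawn amount into Niagara user parameters when a mesh is valid.
; If a VAT data asset is also set, it passes the selected animation's auto-play start and end frames to Niagara.
; All setup happens at construction, with no active event graph logic.
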(fn `UserConstructionScript`
  (bind _niagara (`self.Niagara`))
  (bind _niagara_mesh (`self.Niagara Mesh`)
    (:`then`
      (`NiagaraComponent.SetVariableStaticMesh` _niagara "User.Static Mesh" _niagara_mesh)
      (`NiagaraComponent.SetVariableFloat` _niagara "User.Speed" (`self.Speed`))
      (`NiagaraComponent.SetVariableFloat` _niagara "User.Spread" (`self.Spread`))
      (`NiagaraComponent.SetVariableInt` _niagara "User.Spawn Amount" (`self.Amount`))
      (bind _vat_data_asset (`self.VAT Data Asset`)
        (:`then`
          (bind _autoplaydata (`AnimToTextureInstancePlaybackLibrary.GetAutoPlayDataFromDataAsset` _vat_data_asset (`self.Animation Index`)))
          (`NiagaraComponent.SetVariableFloat` _niagara "User.VAT StartFrame" (`.StartFrame` (break `AnimToTextureAutoPlayData` _autoplaydata)))
          (`NiagaraComponent.SetVariableFloat` _niagara "User.VAT EndFrame" (`.EndFrame` (break `AnimToTextureAutoPlayData` _autoplaydata))))
        (:`else`)))
    (:`else`)))