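; Placer Blueprint that shows a Vertex Animation Texture (VAT) mesh from a data asset, playing the animation selected by AnimationID.
; The construction script adds one instance to an Instanced Static Mesh and swaps each material slot to a dynamic instance.
; Per-instance custom data carries a random time offset plus the animation's play rate and frame range from the data asset.
; An optional Collider flag adds a raised capsule component.
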(fn `UserConstructionScript`
  (bind _instancedstaticmesh (`self.InstancedStaticMesh`))
  (bind _instancedstaticmesh_2 (`self.InstancedStaticMesh`))
  ;[1 1 1] Comment
  ;;[1 1 1] Spawn Static Meshes and give them a dynamic VAT material instance
  (`|ExecutionSequence`
    (:`then_0`
      (`StaticMeshComponent.SetStaticMesh` _instancedstaticmesh_2 (`AnimToTextureDataAsset.BP_GetStaticMesh` (`self.DataAsset`)))
      (`InstancedStaticMeshComponent.AddInstance` _instancedstaticmesh_2 (`KismetMathLibrary.MakeTransform` (0.0 0.0 0.0)) false)
      (for (_ _array_index) (`MeshComponent.GetMaterials` _instancedstaticmesh_2)
        (bind _returnvalue (`PrimitiveComponent.CreateDynamicMaterialInstance` _instancedstaticmesh_2 _array_index (`PrimitiveComponent.GetMaterial` _instancedstaticmesh_2 _array_index) "None"))
        (`PrimitiveComponent.SetMaterial` _instancedstaticmesh_2 _array_index _returnvalue)))
    (:`then_1`
      (bind _autoplaydata (`AnimToTextureInstancePlaybackLibrary.GetAutoPlayDataFromDataAsset` (`self.DataAsset`) (`self.AnimationID`)))
      ;;[1 1 1] Time Offset [0]
      (`InstancedStaticMeshComponent.SetCustomDataValue` _instancedstaticmesh 0 0 (`KismetMathLibrary.RandomFloat`) false)
      ;;[1 1 1] Playrate [1]
      (`InstancedStaticMeshComponent.SetCustomDataValue` _instancedstaticmesh 0 1 (`.PlayRate` (break `AnimToTextureAutoPlayData` _autoplaydata)) false)
      ;;[1 1 1] StartFrame [2]
      (`InstancedStaticMeshComponent.SetCustomDataValue` _instancedstaticmesh 0 2 (`.StartFrame` (break `AnimToTextureAutoPlayData` _autoplaydata)) false)
      ;;[1 1 1] EndFrame [3]
      (`InstancedStaticMeshComponent.SetCustomDataValue` _instancedstaticmesh 0 3 (`.EndFrame` (break `AnimToTextureAutoPlayData` _autoplaydata)) false))
    (:`then_2`
      (if (`self.Collider`)
        (`AddComponent|NODE_AddCapsuleComponent-0` :`RelativeTransform` (`KismetMathLibrary.MakeTransform` (0.0 0.0 90.0)))))))