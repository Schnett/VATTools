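; Renders vertex animation texture (VAT) meshes as instanced static meshes, keeping one component per data asset in a map.
; AddInstance registers and configures any component passed in as static and collision-free, with the asset's mesh and dynamic materials.
; It then adds the instance in world space to the mapped component.
; Per-instance custom data carries a random time offset plus the chosen animation's play rate and frame range.
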(event `Add Instance`
  (params (InstanceTransform :type "Transform Structure (by ref)") (AnimationIndex :type Integer) (DataAsset :type "AnimToTextureDataAsset Object Reference") (`Instaced Static Mesh` :type "InstancedStaticMeshComponent Object Reference") (CastShadow :type Boolean :default true) (EndCullDistance :type Integer :default 20000))
  (bind _returnvalue (`AnimToTextureDataAsset.BP_GetStaticMesh` DataAsset))
  (bind _value (`BlueprintMapLibrary.Map_Find` (`self.VAT Animation Data`) DataAsset))
  (`/Engine/EditorBlueprintResources/StandardMacros.IsValid` `Instaced Static Mesh`
    (:`Is Valid`
      (`BlueprintMapLibrary.Map_Add` (`self.VAT Animation Data`) DataAsset `Instaced Static Mesh`)
      (`InstancedStaticMeshComponent.SetCullDistances` `Instaced Static Mesh` 0 EndCullDistance)
      (`SceneComponent.SetMobility` `Instaced Static Mesh` "Static")
      (set `PrimitiveComponent.bGenerateOverlapEvents` false `Instaced Static Mesh`)
      (`InstancedStaticMeshComponent.SetNumCustomDataFloats` `Instaced Static Mesh` 5)
      (`PrimitiveComponent.SetCollisionEnabled` `Instaced Static Mesh` "NoCollision")
      (`PrimitiveComponent.SetCastShadow` `Instaced Static Mesh` CastShadow)
      (`PrimitiveComponent.SetAffectDistanceFieldLighting` `Instaced Static Mesh` false)
      (`StaticMeshComponent.SetStaticMesh` `Instaced Static Mesh` _returnvalue)
      (for (_array_element _array_index) (`StaticMesh.StaticMaterials` _returnvalue)
        (`PrimitiveComponent.CreateDynamicMaterialInstance` `Instaced Static Mesh` _array_index (break `StaticMaterial` _array_element) "None")))
    (:`Is Not Valid`
      _))
  (bind _returnvalue_2 (`InstancedStaticMeshComponent.AddInstance` _value InstanceTransform true))
  (bind _autoplaydata (`AnimToTextureInstancePlaybackLibrary.GetAutoPlayDataFromDataAsset` DataAsset AnimationIndex))
  ;[1 1 1] Time Offset [0]
  (`InstancedStaticMeshComponent.SetCustomDataValue` _value _returnvalue_2 0 (`KismetMathLibrary.RandomFloat`) false)
  ;[1 1 1] Playrate [1]
  (`InstancedStaticMeshComponent.SetCustomDataValue` _value _returnvalue_2 1 (`.PlayRate` (break `AnimToTextureAutoPlayData` _autoplaydata)) false)
  ;[1 1 1] StartFrame [2]
  (`InstancedStaticMeshComponent.SetCustomDataValue` _value _returnvalue_2 2 (`.StartFrame` (break `AnimToTextureAutoPlayData` _autoplaydata)) false)
  ;[1 1 1] EndFrame [3]
  (`InstancedStaticMeshComponent.SetCustomDataValue` _value _returnvalue_2 3 (`.EndFrame` (break `AnimToTextureAutoPlayData` _autoplaydata)) false))

(fn `UserConstructionScript`)